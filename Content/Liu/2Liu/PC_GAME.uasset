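; PC_GAME appears to be the in-game player controller, handling the countdown HUD, score and server travel.
; On authority, BeginPlay waits briefly, then calls an event, named as a client run, that creates the WBP_CountDown widget.
; Other events push countdown text to that widget and add points to OsuGameInstance.
; CTravel opens an address built from the game instance's ServerIP, a colon and the given LevelName.
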(event Custom|PCUPdateCountDown
  (params (InText2 :type Text))
  (Default|WBPCountUPdate (Variables|Default|GetCountDown) InText2))

(event Custom|PointP
  (params (NewParam :type Integer))
  (bind _asosu_game_instance (Utilities|Casting|CastToOsuGameInstance (Game|GetGameInstance)))
  (bind _output_get (Variables|/Game/Liu/OsuGameInstance.OsuGameInstance_C|SetPoint _asosu_game_instance (+ (Variables|/Game/Liu/OsuGameInstance.OsuGameInstance_C|GetPoint _asosu_game_instance) NewParam)))
  (Development|PrintString (Utilities|String|ToString(Integer) _output_get)))

(event Custom|LiuPCGame_runCliant
  (bind _returnvalue (UserInterface|CreateWidget "/Game/Liu/UI/WBP_CountDown.WBP_CountDown_C"))
  (Variables|Default|SetCountDown _returnvalue)
  (UserInterface|Viewport|AddtoViewport (Variables|Default|GetCountDown) 0))

(event Custom|CTravel
  (params (LevelName :type String))
  (bind _asosu_game_instance (Utilities|Casting|CastToOsuGameInstance (Game|GetGameInstance)))
  (Game|OpenLevel(byName) (Utilities|String|StringToName (Utilities|String|Append (Variables|/Game/Liu/OsuGameInstance.OsuGameInstance_C|GetServerIP _asosu_game_instance) ":" LevelName))))

(event EventBeginPlay
  (Networking|SwitchHasAuthority
    (:Authority
      (Development|PrintString "A")
      (Utilities|FlowControl|Delay 0.2)
      (CallFunction|LiuPCGameRunCliant))))

(event EventTick
  (params (DeltaSeconds :type Float%20%28single-precision%29)))

(fn ConstructionScript)